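; HoldableItem is a Blueprint with one function, AttachToPlayer, that puts an item actor in front of a player as if held in the left or right hand.
; It teleport-free moves the item to a point ahead of the player actor, offset sideways according to the LeftHand flag.
; It then attaches the item to the player actor itself, snapping rotation while using KeepRelative for location and scale.
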(fn `AttachToPlayer`
  (params (ItemActorRef :type "Actor Object Reference") (PlayerActorRef :type "Actor Object Reference") (`LeftHand?` :type Boolean))
  (bind _returnvalue (`Actor.GetActorRightVector` PlayerActorRef))
  (bind _returnvalue_2 (`Actor.K2_GetActorLocation` PlayerActorRef))
  (bind _returnvalue_3 (* (`Actor.GetActorForwardVector` PlayerActorRef) 100))
  (if `LeftHand?`
    (`Actor.K2_SetActorLocation` ItemActorRef (+ _returnvalue_2 _returnvalue_3 (* _returnvalue -30)) false false)
    (else
      (`Actor.K2_SetActorLocation` ItemActorRef (+ _returnvalue_2 _returnvalue_3 (* _returnvalue 30)) false false)))
  (`Actor.K2_AttachToActor` ItemActorRef PlayerActorRef "None" "KeepRelative" "SnapToTarget" "KeepRelative" false)
  (return))