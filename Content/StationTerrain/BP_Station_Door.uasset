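; Sliding double door for a station, opened and closed by a Toggle event with an automatic close five seconds after opening finishes.
; Toggle first flashes the access light green or red from AccessGranted, then recolors the button panel and moves the door whatever that result.
; Open and Close macros loop on short Delays, stepping both panels apart or together along X and counting steps in DoorStatus, without Tick or Timeline.
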(event `Toggle`
  (bind _cube (`self.Cube`))
  (bind _doorstatus (`self.DoorStatus`))
  (bind _buttonpanel2 (`self.ButtonPanel2`))
  ;[1 1 1] Door Toggle
  (if (`self.AccessGranted?`)
    (`PrimitiveComponent.SetMaterial` _cube 0 "/Game/StationTerrain/Mat_Emissive_Green.Mat_Emissive_Green")
    (`KismetSystemLibrary.Delay` 1.2)
    (`PrimitiveComponent.SetMaterial` _cube 0 "/Game/StationTerrain/Mat_Emissive.Mat_Emissive")
    (else
      (`PrimitiveComponent.SetMaterial` _cube 0 "/Game/StationTerrain/Mat_Emissive_Red.Mat_Emissive_Red")
      (`KismetSystemLibrary.Delay` 0.5)
      (`PrimitiveComponent.SetMaterial` _cube 0 "/Game/StationTerrain/Mat_Emissive.Mat_Emissive")
      (`KismetSystemLibrary.Delay` 0.5)
      (`PrimitiveComponent.SetMaterial` _cube 0 "/Game/StationTerrain/Mat_Emissive_Red.Mat_Emissive_Red")
      (`KismetSystemLibrary.Delay` 0.5)
      (`PrimitiveComponent.SetMaterial` _cube 0 "/Game/StationTerrain/Mat_Emissive.Mat_Emissive")))
  (if (`self.Door Open?`)
    (`PrimitiveComponent.SetMaterial` _buttonpanel2 0 "/Game/StationTerrain/Mat_Emissive_Green.Mat_Emissive_Green" :!label _label)
    (if (> _doorstatus 0) :!label _label_2
      (`self.Close Door`)
      (set `self.DoorStatus` (- _doorstatus 1))
      (`KismetSystemLibrary.Delay` 0.05)
      (goto _label_2))
    (else
      (`PrimitiveComponent.SetMaterial` _buttonpanel2 0 "/Game/StationTerrain/Mat_Emissive_Red.Mat_Emissive_Red")
      (if (< _doorstatus 25) :!label _label_3
        (`self.Open Door`)
        (set `self.DoorStatus` (+ _doorstatus 1))
        (`KismetSystemLibrary.Delay` 0.05)
        (goto _label_3)
        (else
          (`KismetSystemLibrary.Delay` 5.0)
          (if (`self.Door Open?`)
            (goto _label)))))))

(fn `Close Door`
  (bind _doorpanel1 (`self.DoorPanel1`))
  (bind _doorpanel2 (`self.DoorPanel2`))
  (bind _result (`/Engine/EditorBlueprintResources/StandardMacros.IncrementFloat` (.x (`SceneComponent.RelativeLocation` _doorpanel1)))
    (:`  `
      (`SceneComponent.K2_SetRelativeLocation` _doorpanel1 (`KismetMathLibrary.MakeVector` _result (.y (`SceneComponent.RelativeLocation` _doorpanel1)) (.z (`SceneComponent.RelativeLocation` _doorpanel1))) false false)
      (bind _result_2 (`/Engine/EditorBlueprintResources/StandardMacros.DecrementFloat` (.x (`SceneComponent.RelativeLocation` _doorpanel2)))
        (:`  `
          (`SceneComponent.K2_SetRelativeLocation` _doorpanel2 (`KismetMathLibrary.MakeVector` _result_2 (.y (`SceneComponent.RelativeLocation` _doorpanel2)) (.z (`SceneComponent.RelativeLocation` _doorpanel2))) false false)
          (set `self.Door Open?` false))))))

(fn `Open Door`
  (bind _doorpanel1 (`self.DoorPanel1`))
  (bind _doorpanel2 (`self.DoorPanel2`))
  (bind _result (`/Engine/EditorBlueprintResources/StandardMacros.DecrementFloat` (.x (`SceneComponent.RelativeLocation` _doorpanel1)))
    (:`  `
      (`SceneComponent.K2_SetRelativeLocation` _doorpanel1 (`KismetMathLibrary.MakeVector` _result (.y (`SceneComponent.RelativeLocation` _doorpanel1)) (.z (`SceneComponent.RelativeLocation` _doorpanel1))) false false)
      (bind _result_2 (`/Engine/EditorBlueprintResources/StandardMacros.IncrementFloat` (.x (`SceneComponent.RelativeLocation` _doorpanel2)))
        (:`  `
          (`SceneComponent.K2_SetRelativeLocation` _doorpanel2 (`KismetMathLibrary.MakeVector` _result_2 (.y (`SceneComponent.RelativeLocation` _doorpanel2)) (.z (`SceneComponent.RelativeLocation` _doorpanel2))) false false)
          (set `self.Door Open?` true))))))

(fn `UserConstructionScript`)