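; Station light Blueprint that switches between white and dim red when the station's emergency state toggles.
; EmergencyToggle stores the Emergency flag and sets the Light component's color to match.
; An unused Fading_2 macro would sweep the light's pitch in a delayed loop during an emergency, wrapping at the upper limit and printing the angle.
; That macro's call is disconnected, so only the color change runs.
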(event `EmergencyToggle`
  (params (`Emergency?` :type Boolean))
  (bind _light (`self.Light`))
  (bind _output_get (set `self.Emergency?` `Emergency?`))
  (if _output_get
    (`LightComponent.SetLightColor` _light (struct :`R` 0.2 :`A` 1.0) true)
    (else
      (`LightComponent.SetLightColor` _light (struct :`R` 1.0 :`G` 1.0 :`B` 1.0 :`A` 1.0) true))))

(fn `UserConstructionScript`)