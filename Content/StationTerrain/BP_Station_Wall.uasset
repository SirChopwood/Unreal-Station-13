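; BP_Station_Wall is a destructible wall piece for the station terrain, built around a Cube component.
; On BeginPlay it applies its Material variable to the cube.
; CheckHP spawns an enlarged explosion emitter at the cube's location and destroys the actor when CurrentHP is zero or below.
; Nothing in this graph changes CurrentHP or calls CheckHP.
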(event `self.ReceiveBeginPlay`
  (`PrimitiveComponent.SetMaterial` (`self.Cube`) 0 (`self.Material`)))

(fn `CheckHP`
  (if (<= (`self.CurrentHP`) 0.0)
    (`GameplayStatics.SpawnEmitterAtLocation` "/Game/StarterContent/Particles/P_Explosion.P_Explosion" (`SceneComponent.K2_GetComponentLocation` (`self.Cube`)) (struct) (3.0 3.0 3.0))
    (`self.K2_DestroyActor`)))

(fn `UserConstructionScript`)