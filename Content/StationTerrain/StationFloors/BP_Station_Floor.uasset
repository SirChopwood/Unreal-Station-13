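; BP_Station_Floor is a destructible station floor piece with configurable tile materials.
; CheckHP spawns a scaled-up explosion emitter at the Cube mesh and destroys the actor once CurrentHP reaches zero or below.
; ReloadTileColours applies the four TileMaterial variables to separate material slots on the Cube.
; BeginPlay and the construction script are empty, and neither function is called within this Blueprint.
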(event `self.ReceiveBeginPlay`)

(fn `CheckHP`
  (if (<= (`self.CurrentHP`) 0.0)
    (`GameplayStatics.SpawnEmitterAtLocation` "/Game/StarterContent/Particles/P_Explosion.P_Explosion" (`SceneComponent.K2_GetComponentLocation` (`self.Cube`)) (struct) (3.0 3.0 3.0))
    (`self.K2_DestroyActor`)))

(fn `Reload Tile Colours`
  (`PrimitiveComponent.SetMaterial` (`self.Cube`) 2 (`self.Tile Material 1`))
  (`PrimitiveComponent.SetMaterial` (`self.Cube`) 3 (`self.Tile Material 2`))
  (`PrimitiveComponent.SetMaterial` (`self.Cube`) 4 (`self.Tile Material 3`))
  (`PrimitiveComponent.SetMaterial` (`self.Cube`) 5 (`self.Tile Material 4`)))

(fn `UserConstructionScript`)