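; Station airlock door with two sliding panels, configurable body and stripe materials, and emissive status lights.
; Toggle flashes green or red access lights from AccessGranted, then opens or closes the door in either case, updating the status lights.
; Open and Close animate the panels with Delay loops that nudge them one unit per step, tracked by DoorStatus.
; An opened door closes automatically after a short wait.
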(event `self.ReceiveBeginPlay`
  (bind _stripecolour (`self.StripeColour`))
  (bind _leftpanel (`self.LeftPanel`))
  (`PrimitiveComponent.SetMaterial` _leftpanel 1 (`self.BodyColour`))
  (`PrimitiveComponent.SetMaterial` (`self.RightPanel`) 1 (`self.BodyColour`))
  (`PrimitiveComponent.SetMaterial` (`self.RightPanel`) 3 _stripecolour)
  (`PrimitiveComponent.SetMaterial` _leftpanel 3 _stripecolour)
  (`PrimitiveComponent.SetMaterial` _leftpanel 7 _stripecolour))

(event `Toggle`
  (bind _leftpanel (`self.LeftPanel`))
  (bind _doorstatus (`self.DoorStatus`))
  (bind _leftpanel_2 (`self.LeftPanel`))
  ;[1 1 1] Door Toggle
  (if (`self.AccessGranted?`)
    (`PrimitiveComponent.SetMaterial` _leftpanel 4 "/Game/StationTerrain/Mat_Emissive_Green.Mat_Emissive_Green")
    (`PrimitiveComponent.SetMaterial` (`self.RightPanel`) 4 "/Game/StationTerrain/Mat_Emissive_Green.Mat_Emissive_Green")
    (`KismetSystemLibrary.Delay` 1.2)
    (`PrimitiveComponent.SetMaterial` _leftpanel 4 "/Game/StationTerrain/Mat_Emissive.Mat_Emissive")
    (`PrimitiveComponent.SetMaterial` (`self.RightPanel`) 4 "/Game/StationTerrain/Mat_Emissive.Mat_Emissive")
    (else
      (`PrimitiveComponent.SetMaterial` _leftpanel 4 "/Game/StationTerrain/Mat_Emissive_Red.Mat_Emissive_Red")
      (`PrimitiveComponent.SetMaterial` (`self.RightPanel`) 4 "/Game/StationTerrain/Mat_Emissive_Red.Mat_Emissive_Red")
      (`KismetSystemLibrary.Delay` 0.5)
      (`PrimitiveComponent.SetMaterial` _leftpanel 4 "/Game/StationTerrain/Mat_Emissive.Mat_Emissive")
      (`PrimitiveComponent.SetMaterial` (`self.RightPanel`) 4 "/Game/StationTerrain/Mat_Emissive.Mat_Emissive")
      (`KismetSystemLibrary.Delay` 0.5)
      (`PrimitiveComponent.SetMaterial` _leftpanel 4 "/Game/StationTerrain/Mat_Emissive_Red.Mat_Emissive_Red")
      (`PrimitiveComponent.SetMaterial` (`self.RightPanel`) 4 "/Game/StationTerrain/Mat_Emissive_Red.Mat_Emissive_Red")
      (`KismetSystemLibrary.Delay` 0.5)
      (`PrimitiveComponent.SetMaterial` _leftpanel 4 "/Game/StationTerrain/Mat_Emissive.Mat_Emissive")
      (`PrimitiveComponent.SetMaterial` (`self.RightPanel`) 4 "/Game/StationTerrain/Mat_Emissive.Mat_Emissive")))
  (if (`self.Door Open?`)
    (`PrimitiveComponent.SetMaterial` _leftpanel_2 5 "/Game/StationTerrain/Mat_Emissive_Red.Mat_Emissive_Red" :!label _label)
    (`PrimitiveComponent.SetMaterial` _leftpanel_2 6 "/Game/StationTerrain/Mat_Emissive_Red.Mat_Emissive_Red")
    (if (> _doorstatus 0) :!label _label_2
      (`self.Close Door`)
      (set `self.DoorStatus` (- _doorstatus 1))
      (`KismetSystemLibrary.Delay` 0.05)
      (goto _label_2))
    (else
      (`PrimitiveComponent.SetMaterial` _leftpanel_2 5 "/Game/StationTerrain/Mat_Emissive_Green.Mat_Emissive_Green")
      (`PrimitiveComponent.SetMaterial` _leftpanel_2 6 "/Game/StationTerrain/Mat_Emissive_Green.Mat_Emissive_Green")
      (if (< _doorstatus 25) :!label _label_3
        (`self.Open Door`)
        (set `self.DoorStatus` (+ _doorstatus 1))
        (`KismetSystemLibrary.Delay` 0.05)
        (goto _label_3)
        (else
          (`KismetSystemLibrary.Delay` 5.0)
          (if (`self.Door Open?`)
            (goto _label)))))))

(fn `Close Door`
  (bind _rightpanel (`self.RightPanel`))
  (bind _leftpanel (`self.LeftPanel`))
  (bind _result (`/Engine/EditorBlueprintResources/StandardMacros.IncrementFloat` (.x (`SceneComponent.RelativeLocation` _rightpanel)))
    (:`  `
      (`SceneComponent.K2_SetRelativeLocation` _rightpanel (`KismetMathLibrary.MakeVector` _result (.y (`SceneComponent.RelativeLocation` _rightpanel)) (.z (`SceneComponent.RelativeLocation` _rightpanel))) false false)
      (bind _result_2 (`/Engine/EditorBlueprintResources/StandardMacros.DecrementFloat` (.x (`SceneComponent.RelativeLocation` _leftpanel)))
        (:`  `
          (`SceneComponent.K2_SetRelativeLocation` _leftpanel (`KismetMathLibrary.MakeVector` _result_2 (.y (`SceneComponent.RelativeLocation` _leftpanel)) (.z (`SceneComponent.RelativeLocation` _leftpanel))) false false)
          (set `self.Door Open?` false))))))

(fn `Open Door`
  (bind _rightpanel (`self.RightPanel`))
  (bind _leftpanel (`self.LeftPanel`))
  (bind _result (`/Engine/EditorBlueprintResources/StandardMacros.DecrementFloat` (.x (`SceneComponent.RelativeLocation` _rightpanel)))
    (:`  `
      (`SceneComponent.K2_SetRelativeLocation` _rightpanel (`KismetMathLibrary.MakeVector` _result (.y (`SceneComponent.RelativeLocation` _rightpanel)) (.z (`SceneComponent.RelativeLocation` _rightpanel))) false false)
      (bind _result_2 (`/Engine/EditorBlueprintResources/StandardMacros.IncrementFloat` (.x (`SceneComponent.RelativeLocation` _leftpanel)))
        (:`  `
          (`SceneComponent.K2_SetRelativeLocation` _leftpanel (`KismetMathLibrary.MakeVector` _result_2 (.y (`SceneComponent.RelativeLocation` _leftpanel)) (.z (`SceneComponent.RelativeLocation` _leftpanel))) false false)
          (set `self.Door Open?` true))))))

(fn `UserConstructionScript`)