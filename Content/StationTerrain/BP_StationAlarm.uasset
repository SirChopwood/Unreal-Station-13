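; Station alarm Blueprint that toggles the station's emergency state and its warning audio.
; ToggleAlarm plays an attenuated intercepted-comms sound at its cube and waits before switching on, or destroys the stored alarm sound when switching off.
; It then passes the new state to every BP_Station_Light through EmergencyToggle.
; When active, a delayed spawn inside that light loop starts the alarm sound and stores it for later removal.
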(event `ToggleAlarm`
  (if (`self.Alarm Active`)
    (`ActorComponent.K2_DestroyComponent` (`self.SoundRef`))
    (set `self.Alarm Active` false)
    (else
      (`GameplayStatics.SpawnSoundAtLocation` "/Game/StationTerrain/SFX_AI_CommsIntercepted.SFX_AI_CommsIntercepted" (`SceneComponent.K2_GetComponentLocation` (`self.Cube`)) (struct) 2.0 1.0 0.0 (`self.Attenuation`) null)
      (`KismetSystemLibrary.Delay` 3.8)
      (bind _output_get (set `self.Alarm Active` true))))
  (bind _outactors (`GameplayStatics.GetAllActorsOfClass` "/Game/StationTerrain/BP_Station_Light.BP_Station_Light_C"))
  (for _array_element _outactors
    (`/Game/StationTerrain/BP_Station_Light.EmergencyToggle` _array_element (`self.Alarm Active`))
    (if _output_get
      (`KismetSystemLibrary.Delay` 2.6)
      (bind _returnvalue (`GameplayStatics.SpawnSoundAtLocation` "/Game/StationTerrain/SFX_StationAlarm.SFX_StationAlarm" (0.0 0.0 0.0) (struct) 0.8 1.0 0.0 null null false))
      (set `self.SoundRef` _returnvalue))))

(fn `UserConstructionScript`)